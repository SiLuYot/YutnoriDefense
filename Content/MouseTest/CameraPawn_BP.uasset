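; CameraPawn_BP is a camera pawn that pans along world X and Y from movement axis input or screen-edge mouse scrolling.
; MoveForward and MoveRight pass nonzero axis values to AddMovementInput, otherwise deriving the scale from mouse position.
; CalculateScale returns zero in the middle of the viewport and ramps linearly to ±1 across the outer 10% bands.
; Mouse Y is inverted so the top edge moves forward.
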(event `InputAxis|MoveForward`
  (params (AxisValue :type "Float (single-precision)"))
  (bind (_returnvalue_x _returnvalue_y) (`KismetMathLibrary.BreakVector2D` (`WidgetLayoutLibrary.GetViewportSize`)))
  (if (== AxisValue 0.0)
    (bind _scale (`self.CalculateScale` (- _returnvalue_y (`.LocationY` (`PlayerController.GetMousePosition` (`GameplayStatics.GetPlayerController` 0)))) _returnvalue_y))
    (`self.AddMovementInput` (1.0 0.0 0.0) _scale)
    (else
      (`self.AddMovementInput` (1.0 0.0 0.0) AxisValue))))

(event `InputAxis|MoveRight`
  (params (AxisValue :type "Float (single-precision)"))
  (bind _returnvalue_x (`KismetMathLibrary.BreakVector2D` (`WidgetLayoutLibrary.GetViewportSize`)))
  (if (== AxisValue 0.0)
    (bind _scale (`self.CalculateScale` (`PlayerController.GetMousePosition` (`GameplayStatics.GetPlayerController` 0)) _returnvalue_x))
    (`self.AddMovementInput` (0.0 1.0 0.0) _scale)
    (else
      (`self.AddMovementInput` (0.0 1.0 0.0) AxisValue))))

(fn `CalculateScale`
  (params (MouseAxisValue :type "Float (double-precision)") (ViewportAxisValue :type "Float (double-precision)"))
  (returns (Scale :type "Float (double-precision)"))
  (bind _returnvalue (* ViewportAxisValue 0.9))
  (bind _returnvalue_2 (* ViewportAxisValue 0.1))
  (if (> MouseAxisValue _returnvalue)
    (return (/ (- MouseAxisValue _returnvalue) _returnvalue_2))
    (elif (< MouseAxisValue _returnvalue_2)
      (return (+ (/ MouseAxisValue _returnvalue_2) -1.0))
      (else
        (return 0.0)))))

(fn `UserConstructionScript`)